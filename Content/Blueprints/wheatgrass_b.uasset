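; Wheatgrass foliage actor that rustles when the player brushes through it.
; Capsule begin and end overlaps with Player-tagged actors set an overlap flag and call the shake event.
; On entry, a DoOnce gate plays the audio and runs a timeline that rotates the static mesh in pitch.
; Leaving the capsule resets the gate so the next entry triggers it again.
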(event `ShakeTIme`
  (if (`self.Overlapped`)
    (`/Engine/EditorBlueprintResources/StandardMacros.DoOnce` false :!label _label
      (:`Completed`
        (`AudioComponent.Play` (`self.Audio`) 0.0)
        (bind (_direction _newtrack_0) (`Timeline|Shake` :!via `PlayFromStart`)
          (:`Update`
            (`SceneComponent.K2_SetRelativeRotation` (`self.StaticMesh`) (`KismetMathLibrary.MakeRotator` 0.0 _newtrack_0) false false)))))
    (else
      (goto _label :!via `Reset`))))

(event `self.Capsule.OnComponentBeginOverlap`
  (params (OverlappedComponent :type "PrimitiveComponent Object Reference") (OtherActor :type "Actor Object Reference") (OtherComp :type "PrimitiveComponent Object Reference") (OtherBodyIndex :type Integer) (bFromSweep :type Boolean) (SweepResult :type "HitResult Structure (by ref)"))
  (if (`self.ActorHasTag` OtherActor "Player")
    (set `self.Overlapped` true)
    (`self.ShakeTIme`)))

(event `self.Capsule.OnComponentEndOverlap`
  (params (OverlappedComponent :type "PrimitiveComponent Object Reference") (OtherActor :type "Actor Object Reference") (OtherComp :type "PrimitiveComponent Object Reference") (OtherBodyIndex :type Integer))
  (if (`self.ActorHasTag` OtherActor "Player")
    (set `self.Overlapped` false)
    (`self.ShakeTIme`)))

(fn `UserConstructionScript`)